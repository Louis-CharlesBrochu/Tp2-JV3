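; BP_RandomDoor randomizes a door number from 1 to 3 for each of four levels.
; Its RandomDoor function writes each roll to the PorteLv1 to PorteLv4 variables on BP_GameInstance, stopping if that cast fails.
; The rounding step is redundant, as the rolls are already integers.
; A red debug print shows the four values concatenated.
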(fn `RandomDoor`
  (bind _asbp_game_instance (cast `/Game/Game/Blueprints/BP_GameInstance` (`GameplayStatics.GetGameInstance` null)))
  ; Set Nombre random + arondisement
  (bind _output_get (set `/Game/Game/Blueprints/BP_GameInstance.PorteLv1` (`KismetMathLibrary.Conv_IntToDouble` (`KismetMathLibrary.Round` (`KismetMathLibrary.Conv_IntToDouble` (`KismetMathLibrary.RandomIntegerInRange` 1 3)))) _asbp_game_instance))
  (bind _output_get_2 (set `/Game/Game/Blueprints/BP_GameInstance.PorteLv2` (`KismetMathLibrary.Conv_IntToDouble` (`KismetMathLibrary.Round` (`KismetMathLibrary.Conv_IntToDouble` (`KismetMathLibrary.RandomIntegerInRange` 1 3)))) _asbp_game_instance))
  (bind _output_get_3 (set `/Game/Game/Blueprints/BP_GameInstance.PorteLv3` (`KismetMathLibrary.Conv_IntToDouble` (`KismetMathLibrary.Round` (`KismetMathLibrary.Conv_IntToDouble` (`KismetMathLibrary.RandomIntegerInRange` 1 3)))) _asbp_game_instance))
  (bind _output_get_4 (set `/Game/Game/Blueprints/BP_GameInstance.PorteLv4` (`KismetMathLibrary.Conv_IntToDouble` (`KismetMathLibrary.Round` (`KismetMathLibrary.Conv_IntToDouble` (`KismetMathLibrary.RandomIntegerInRange` 1 3)))) _asbp_game_instance))
  ; Debug
  (`KismetSystemLibrary.PrintText` null (`KismetTextLibrary.Conv_StringToText` (`KismetStringLibrary.Concat_StrStr` (`KismetStringLibrary.Conv_DoubleToString` _output_get) (`KismetStringLibrary.Conv_DoubleToString` _output_get_2) (`KismetStringLibrary.Conv_DoubleToString` _output_get_3) (`KismetStringLibrary.Conv_DoubleToString` _output_get_4))) true true (struct :`R` 1.0 :`A` 1.0) 10.0))