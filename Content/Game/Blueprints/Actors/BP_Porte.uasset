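; BP_Porte is a colored door that opens only if its color is the correct one for the current level.
; BeginPlay sets door and frame materials from Couleur and caches BP_GameInstance; a trigger overlap shows or hides a widget.
; Interact checks Couleur against that level's PorteLv value across four levels, toggling a timeline rotation on a match.
; A mismatch damages the player through BP_PlayerState's health component; the open sound plays only on the level 1 match.
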(event `self.Interact Trigger.OnComponentBeginOverlap`
  (params (OverlappedComponent :type "PrimitiveComponent Object Reference") (OtherActor :type "Actor Object Reference") (OtherComp :type "PrimitiveComponent Object Reference") (OtherBodyIndex :type Integer) (bFromSweep :type Boolean) (SweepResult :type "HitResult Structure (by ref)"))
  (`SceneComponent.SetVisibility` (`self.Widget`) true false))

(event `self.Interact Trigger.OnComponentEndOverlap`
  (params (OverlappedComponent :type "PrimitiveComponent Object Reference") (OtherActor :type "Actor Object Reference") (OtherComp :type "PrimitiveComponent Object Reference") (OtherBodyIndex :type Integer))
  (`SceneComponent.SetVisibility` (`self.Widget`) false false))

(event `self.ReceiveBeginPlay`
  (bind _couleur (`self.Couleur`))
  (bind _cadredeporte (`self.CadredePorte`))
  ;[0 0 1 1] Changement Couleur Porte
  (`|ExecutionSequence`
    (:`then_0`
      (if (== _couleur 1.0)
        (`PrimitiveComponent.SetMaterial` _cadredeporte 0 "/Game/Game/Materials/M_Rouge.M_Rouge")
        (`PrimitiveComponent.SetMaterial` (`self.Porte`) 0 "/Game/Game/Materials/M_Rouge.M_Rouge")))
    (:`then_1`
      (if (== _couleur 2.0)
        (`PrimitiveComponent.SetMaterial` _cadredeporte 0 "/Game/Game/Materials/M_Vert.M_Vert")
        (`PrimitiveComponent.SetMaterial` (`self.Porte`) 0 "/Game/Game/Materials/M_Vert.M_Vert")))
    (:`then_2`
      (if (== _couleur 3.0)
        (`PrimitiveComponent.SetMaterial` (`self.Porte`) 0 "/Game/Game/Materials/M_Bleue.M_Bleue")
        (`PrimitiveComponent.SetMaterial` _cadredeporte 0 "/Game/Game/Materials/M_Bleue.M_Bleue")))
    (:`then_3`
      (bind _asbp_game_instance (cast `/Game/Game/Blueprints/BP_GameInstance` (`GameplayStatics.GetGameInstance`))))))

(event `MouvementPorte`
  ; Verification
)

(event `/Game/Game/Blueprints/Interfaces/BPI_Interact.Interact`
  ; Verification
  (bind _level (`/Game/Game/Blueprints/BP_GameInstance.Level` (stale `self.ReceiveBeginPlay` _asbp_game_instance)))
  (if (and (== _level 1.0) (== (`self.Couleur`) (`/Game/Game/Blueprints/BP_GameInstance.PorteLv1` (stale `self.ReceiveBeginPlay` _asbp_game_instance))))
    (`GameplayStatics.PlaySoundAtLocation` "/Game/Game/Audio/SFX/MC_sons/SC_Open-door.SC_Open-door" (0.0 0.0 0.0) (struct) 1.0 1.0 0.0 null null null null)
    ;[0 1 0.009034] Bonne porte
    (`/Engine/EditorBlueprintResources/StandardMacros.FlipFlop` :!label _label
      (:`A`
        (bind (_direction _axez) (`Timeline|AnimationPorte` :!label _label_2)
          (:`Update`
            (`SceneComponent.K2_SetRelativeRotation` (`self.Porte`) (`KismetMathLibrary.MakeRotator` 0.0 0.0 _axez) false false))))
      (:`B`
        (goto _label_2 :!via `Reverse`)))
    (elif (and (== _level 2.0) (== (`self.Couleur`) (`/Game/Game/Blueprints/BP_GameInstance.PorteLv2` (stale `self.ReceiveBeginPlay` _asbp_game_instance))))
      (goto _label)
      (elif (and (== _level 3.0) (== (`self.Couleur`) (`/Game/Game/Blueprints/BP_GameInstance.PorteLv3` (stale `self.ReceiveBeginPlay` _asbp_game_instance))))
        (goto _label)
        (elif (and (== _level 4.0) (== (`self.Couleur`) (`/Game/Game/Blueprints/BP_GameInstance.PorteLv4` (stale `self.ReceiveBeginPlay` _asbp_game_instance))))
          (goto _label)
          (else
            ;[1 0 0] Mauvaise porte
            (bind _outactors (`GameplayStatics.GetAllActorsOfClass` "/Game/Game/Blueprints/Pawns_Characters/Player/BP_ThirdPersonCharacter.BP_ThirdPersonCharacter_C"))
            (bind _asbp_player_state (cast `/Game/Game/Blueprints/PlayerStates/BP_PlayerState` (`Pawn.PlayerState` (`|GetArrayItem` _outactors))))
            (`/Game/Game/Blueprints/Components/AC_Health.TakeDamage` (`/Game/Game/Blueprints/PlayerStates/BP_PlayerState.AC_Health` _asbp_player_state) 25.0)
            (`GameplayStatics.PlaySound2D` "/Game/Game/Audio/SFX/MC_sons/SC_hero-hurt.SC_hero-hurt" 1.0 1.0 0.0 null null)))))))

(fn `UserConstructionScript`)