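; BP_MurPortes is a level-exit actor that moves the player on to the next level when its Collision component is overlapped.
; It checks that CurrentHealthGI in BP_GameInstance is above zero, then waits briefly before reading the Level value.
; That value selects which of Lvl2, Lvl3 or Lvl4 opens by object reference.
; The overlapping actor is never checked, and Level is only read, not changed.
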(event `self.Collision.OnComponentBeginOverlap`
  (params (OverlappedComponent :type "PrimitiveComponent Object Reference") (OtherActor :type "Actor Object Reference") (OtherComp :type "PrimitiveComponent Object Reference") (OtherBodyIndex :type Integer) (bFromSweep :type Boolean) (SweepResult :type "HitResult Structure (by ref)"))
  (bind _asbp_game_instance (cast `/Game/Game/Blueprints/BP_GameInstance` (`GameplayStatics.GetGameInstance`)))
  (if (> (`/Game/Game/Blueprints/BP_GameInstance.CurrentHealth_GI` _asbp_game_instance) 0.0)
    (`KismetSystemLibrary.Delay` 1.0)
    (bind _asbp_game_instance_2 (cast `/Game/Game/Blueprints/BP_GameInstance` (`GameplayStatics.GetGameInstance`)))
    (`|ExecutionSequence`
      (:`then_0`
        (bind _level (`/Game/Game/Blueprints/BP_GameInstance.Level` _asbp_game_instance_2))
        (if (== _level 1.0)
          (`GameplayStatics.OpenLevelBySoftObjectPtr` "/Game/Game/Maps/Lvl2.Lvl2")))
      (:`then_1`
        (if (== _level 2.0)
          (`GameplayStatics.OpenLevelBySoftObjectPtr` "/Game/Game/Maps/Lvl3.Lvl3")))
      (:`then_2`
        (if (== _level 3.0)
          (`GameplayStatics.OpenLevelBySoftObjectPtr` "/Game/Game/Maps/Lvl4.Lvl4"))))))

(fn `UserConstructionScript`)