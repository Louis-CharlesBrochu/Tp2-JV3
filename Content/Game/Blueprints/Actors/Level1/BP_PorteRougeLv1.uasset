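; BP_PorteRougeLv1 is the red door of Level 1, showing an interaction prompt widget while something overlaps its trigger.
; The MouvementPorteRouge event checks PorteLv1 on the game instance and, when set, alternately opens and closes the door through a FlipFlop and a yaw-rotation timeline.
; Otherwise it damages the first third-person character found, via the health component on its PlayerState.
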(event `MouvementPorteRouge`
  (bind _asbp_game_instance (cast `/Game/Game/Blueprints/BP_GameInstance` (`GameplayStatics.GetGameInstance`)))
  (if (== (`/Game/Game/Blueprints/BP_GameInstance.PorteLv1` _asbp_game_instance) 1.0)
    (`/Engine/EditorBlueprintResources/StandardMacros.FlipFlop`
      (:`A`
        (bind (_direction _axez) (`Timeline|AnimationPorte` :!label _label)
          (:`Update`
            (`SceneComponent.K2_SetRelativeRotation` (`self.Porte`) (`KismetMathLibrary.MakeRotator` 0.0 0.0 _axez) false false))))
      (:`B`
        (goto _label :!via `Reverse`)))
    (else
      (bind _outactors (`GameplayStatics.GetAllActorsOfClass` "/Game/Game/Blueprints/Pawns_Characters/Player/BP_ThirdPersonCharacter.BP_ThirdPersonCharacter_C"))
      (bind _asbp_player_state (cast `/Game/Game/Blueprints/PlayerStates/BP_PlayerState` (`Pawn.PlayerState` (`|GetArrayItem` _outactors))))
      (`/Game/Game/Blueprints/Components/AC_Health.TakeDamage` (`/Game/Game/Blueprints/PlayerStates/BP_PlayerState.AC_Health` _asbp_player_state) 25.0))))

(event `self.Interact Trigger.OnComponentBeginOverlap`
  (params (OverlappedComponent :type "PrimitiveComponent Object Reference") (OtherActor :type "Actor Object Reference") (OtherComp :type "PrimitiveComponent Object Reference") (OtherBodyIndex :type Integer) (bFromSweep :type Boolean) (SweepResult :type "HitResult Structure (by ref)"))
  (`SceneComponent.SetVisibility` (`self.Widget`) true false))

(event `self.Interact Trigger.OnComponentEndOverlap`
  (params (OverlappedComponent :type "PrimitiveComponent Object Reference") (OtherActor :type "Actor Object Reference") (OtherComp :type "PrimitiveComponent Object Reference") (OtherBodyIndex :type Integer))
  (`SceneComponent.SetVisibility` (`self.Widget`) false false))

(fn `UserConstructionScript`)