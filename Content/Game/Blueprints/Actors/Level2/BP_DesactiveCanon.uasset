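; Level 2 interactable lever actor that deactivates a cannon, going by its name and dispatcher.
; Interact works only while ShieldActive is true: it fires the DestroyCanon dispatcher and clears the flag, preventing repeat use.
; The Levier timeline then drives a MoveComponentTo on the Cylinder to animate the lever, stopping it when finished.
; Overlap events on CharacterDetectror show and hide a widget as things enter and leave.
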(event `/Game/Game/Blueprints/Interfaces/BPI_Interact.Interact`
  (if (`self.shield_active`)
    (`self.destroy_canon`)
    (set `self.shield_active` false)
    (`Timeline|levier` :!via `PlayFromStart`
      (:`Update`
        (`KismetSystemLibrary.MoveComponentTo` (`self.Cylinder`) (0.0 13.0 -10.0) (struct :`Roll` 90.0) :!label _label))
      (:`Finished`
        (goto _label :!via `Stop`)))))

(event `self.character detectror.OnComponentBeginOverlap`
  (params (OverlappedComponent :type "PrimitiveComponent Object Reference") (OtherActor :type "Actor Object Reference") (OtherComp :type "PrimitiveComponent Object Reference") (OtherBodyIndex :type Integer) (bFromSweep :type Boolean) (SweepResult :type "HitResult Structure (by ref)"))
  (`SceneComponent.SetVisibility` (`self.Widget`) true false))

(event `self.character detectror.OnComponentEndOverlap`
  (params (OverlappedComponent :type "PrimitiveComponent Object Reference") (OtherActor :type "Actor Object Reference") (OtherComp :type "PrimitiveComponent Object Reference") (OtherBodyIndex :type Integer))
  (`SceneComponent.SetVisibility` (`self.Widget`) false false))

(fn `UserConstructionScript`)