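; Level 2 cannon actor that turns toward the player and fires projectiles when it sees them.
; PawnSensing triggers aiming at the third-person character, then spawns BP_Projectile from the arrow component after a short delay, with an extra wind-up before the first shot.
; On BeginPlay it binds to an event on the BP_DesactiveCanon found in the level, which destroys the cannon when fired.
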(event `self.ReceiveBeginPlay`
  (bind _returnvalue (`GameplayStatics.GetActorOfClass` "/Game/Game/Blueprints/Actors/Level2/BP_DesactiveCanon.BP_DesactiveCanon_C"))
  (add `/Game/Game/Blueprints/Actors/Level2/BP_DesactiveCanon.destroy_canon` _returnvalue (delegate `destroy`)))

(event `destroy`
  (`self.K2_DestroyActor`))

(event `self.PawnSensing.OnSeePawn`
  (params (Pawn :type "Pawn Object Reference"))
  ; tire projectile sur le joueur
  (if (`self.start`)
    (`KismetSystemLibrary.Delay` 1.0))
  (cast `/Game/Game/Blueprints/Pawns_Characters/Player/BP_ThirdPersonCharacter` Pawn)
  (`self.K2_SetActorRotation` (`KismetMathLibrary.FindLookAtRotation` (`self.K2_GetActorLocation`) (`self.K2_GetActorLocation` Pawn)))
  (`KismetSystemLibrary.Delay` 0.2)
  (set `self.start` false)
  (`|SpawnActorFromClass` "/Game/Game/Blueprints/Actors/Level2/BP_Projectile.BP_Projectile_C" (`SceneComponent.K2_GetComponentToWorld` (`self.flèche`)) "Undefined" "MultiplyWithRoot" null null))

(fn `UserConstructionScript`)