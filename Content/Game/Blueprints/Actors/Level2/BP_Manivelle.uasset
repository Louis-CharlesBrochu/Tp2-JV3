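; BP_Manivelle is a Level 2 crank lever that the player can use once while ShieldActive is true.
; Interact calls DestroyCanon, clears ShieldActive, plays a 2D sound, then runs the Levier timeline, whose updates drive a MoveComponentTo that moves and rotates the Manivelle component.
; The CharacterDetectror overlap shows and hides the EInteract prompt for BP_ThirdPersonCharacter.
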(event `/Game/Game/Blueprints/Interfaces/BPI_Interact.Interact`
  ; interaction avec le levier et animation
  (if (`self.shield_active`)
    (`self.destroy_canon`)
    (set `self.shield_active` false)
    (`GameplayStatics.SpawnSound2D` "/Game/Game/Blueprints/Actors/Level2/5.5" 1.0 1.0 0.0 null)
    (`Timeline|levier`
      (:`Update`
        (`KismetSystemLibrary.MoveComponentTo` (`self.manivelle`) (0.0 13.0 -10.0) (struct :`Roll` 90.0) :!label _label))
      (:`Finished`
        (goto _label :!via `Stop`)))))

(event `self.character detectror.OnComponentBeginOverlap`
  (params (OverlappedComponent :type "PrimitiveComponent Object Reference") (OtherActor :type "Actor Object Reference") (OtherComp :type "PrimitiveComponent Object Reference") (OtherBodyIndex :type Integer) (bFromSweep :type Boolean) (SweepResult :type "HitResult Structure (by ref)"))
  ; apparition du widget
  (cast `/Game/Game/Blueprints/Pawns_Characters/Player/BP_ThirdPersonCharacter` OtherActor)
  (`SceneComponent.SetVisibility` (`self.e_Interact`) true false))

(event `self.character detectror.OnComponentEndOverlap`
  (params (OverlappedComponent :type "PrimitiveComponent Object Reference") (OtherActor :type "Actor Object Reference") (OtherComp :type "PrimitiveComponent Object Reference") (OtherBodyIndex :type Integer))
  ; apparition du widget
  (cast `/Game/Game/Blueprints/Pawns_Characters/Player/BP_ThirdPersonCharacter` OtherActor)
  (`SceneComponent.SetVisibility` (`self.e_Interact`) false false))

(fn `UserConstructionScript`)