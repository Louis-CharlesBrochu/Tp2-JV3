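; BP_MurPiqueLVL4 is a spiked wall hazard for Level 4 that damages the player on contact.
; Overlapping its Collision component casts to BP_ThirdPersonCharacter and its BP_PlayerState, then applies heavy damage through the ACHealth component.
; An unconnected delayed timeline would push the wall along world X, but it never runs, so this Blueprint does not move the wall.
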(event `self.ReceiveBeginPlay`)

(event `self.collision.OnComponentBeginOverlap`
  (params (OverlappedComponent :type "PrimitiveComponent Object Reference") (OtherActor :type "Actor Object Reference") (OtherComp :type "PrimitiveComponent Object Reference") (OtherBodyIndex :type Integer) (bFromSweep :type Boolean) (SweepResult :type "HitResult Structure (by ref)"))
  ; Enlever Vie
  (`KismetSystemLibrary.PrintText` "Collision")
  (bind _asbp_third_person_character (cast `/Game/Game/Blueprints/Pawns_Characters/Player/BP_ThirdPersonCharacter` OtherActor))
  (bind _asbp_player_state (cast `/Game/Game/Blueprints/PlayerStates/BP_PlayerState` (`Pawn.PlayerState` _asbp_third_person_character)))
  (`/Game/Game/Blueprints/Components/AC_Health.TakeDamage` (`/Game/Game/Blueprints/PlayerStates/BP_PlayerState.AC_Health` _asbp_player_state) 100.0))

(fn `UserConstructionScript`)