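; BP_Interaction is an interactable actor with a configurable mesh, sphere trigger and UI component.
; The construction script applies the mesh, trigger radius and component offsets from variables; TriggerRotation actually sets the trigger's location.
; Trigger overlaps add or remove the actor on BP_ThirdPersonCharacter, and ToggleUi sets prompt visibility.
; Interact stores the character, prints a debug string and fires the StartWall dispatcher.
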(event `self.Interact Trigger.OnComponentBeginOverlap`
  (params (OverlappedComponent :type "PrimitiveComponent Object Reference") (OtherActor :type "Actor Object Reference") (OtherComp :type "PrimitiveComponent Object Reference") (OtherBodyIndex :type Integer) (bFromSweep :type Boolean) (SweepResult :type "HitResult Structure (by ref)"))
  ; Trigger Overlap
  (bind _asbp_third_person_character (cast `/Game/Game/Blueprints/Pawns_Characters/Player/BP_ThirdPersonCharacter` OtherActor))
  (`/Game/Game/Blueprints/Pawns_Characters/Player/BP_ThirdPersonCharacter.AddInteraction` _asbp_third_person_character self))

(event `self.Interact Trigger.OnComponentEndOverlap`
  (params (OverlappedComponent :type "PrimitiveComponent Object Reference") (OtherActor :type "Actor Object Reference") (OtherComp :type "PrimitiveComponent Object Reference") (OtherBodyIndex :type Integer))
  ; Trigger Overlap
  (bind _asbp_third_person_character (cast `/Game/Game/Blueprints/Pawns_Characters/Player/BP_ThirdPersonCharacter` OtherActor))
  (`/Game/Game/Blueprints/Pawns_Characters/Player/BP_ThirdPersonCharacter.RemoveInteraction` _asbp_third_person_character self))

(fn `Interact`
  (params (Character :type "/Game/Game/Blueprints/Actors/BP_Interaction Object Reference"))
  (locals (NewLocalVar :type "/Game/Game/Blueprints/Actors/BP_Interaction Object Reference"))
  ; Interaction
  (set `self.InteractCharacter` Character)
  (`KismetSystemLibrary.PrintString` "Interagie")
  (`self.startWall`))

(fn `SetupMesh`
  ; Setup Mesh - Static Mesh position
  (`StaticMeshComponent.SetStaticMesh` (`self.Interact Mesh`) (`self.InteractionMesh`))
  (`SceneComponent.K2_SetRelativeTransform` (`self.Interact Mesh`) (`self.MeshTransform`) false false))

(fn `SetupTrigger`
  ; Setup Trigger
  (`SphereComponent.SetSphereRadius` (`self.Interact Trigger`) (`self.TriggerRadius`) true)
  (`SceneComponent.K2_SetRelativeLocation` (`self.Interact Trigger`) (`self.TriggerRotation`) false false))

(fn `SetupUi`
  ; Setup Ui set location offset
  (`SceneComponent.K2_SetRelativeLocation` (`self.Interact Ui`) (`self.UiLocation`) false false))

(fn `ToggleUi`
  (params (bVisible :type Boolean))
  ; Set Visibility
  (`SceneComponent.SetVisibility` (`self.Interact Ui`) bVisible false))

(fn `UserConstructionScript`
  ; Construction Script Setup Interaction
  (`self.SetupMesh`)
  (`self.SetupTrigger`)
  (`self.SetupUi`))