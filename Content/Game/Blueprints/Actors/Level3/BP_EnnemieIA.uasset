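; Level 3 enemy AI character that chases the player on sight and damages them on contact.
; PawnSensing triggers an AI MoveTo toward the player, then plays a pistol-fire montage on arrival.
; CanAttack locks out attacks for the montage's duration, while Tick halts movement.
; Separately, sphere overlap with the player deals heavy damage through the PlayerState's health component, independent of the animation.
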(event `self.SphereCollision.OnComponentBeginOverlap`
  (params (OverlappedComponent :type "PrimitiveComponent Object Reference") (OtherActor :type "Actor Object Reference") (OtherComp :type "PrimitiveComponent Object Reference") (OtherBodyIndex :type Integer) (bFromSweep :type Boolean) (SweepResult :type "HitResult Structure (by ref)"))
  (bind _asbp_third_person_character (cast `/Game/Game/Blueprints/Pawns_Characters/Player/BP_ThirdPersonCharacter` OtherActor))
  (`KismetSystemLibrary.PrintString` "collision")
  (bind _asbp_player_state (cast `/Game/Game/Blueprints/PlayerStates/BP_PlayerState` (`Pawn.PlayerState` _asbp_third_person_character)))
  (`KismetSystemLibrary.PrintString` "Hello")
  (`/Game/Game/Blueprints/Components/AC_Health.TakeDamage` (`/Game/Game/Blueprints/PlayerStates/BP_PlayerState.AC_Health` _asbp_player_state) 150.0))

(event `self.ReceiveTick`
  (params (DeltaSeconds :type "Float (single-precision)"))
  (if (not (`self.canAttack?`))
    (`MovementComponent.StopMovementImmediately` (`self.CharacterMovement`))))

(event `self.PawnSensing.OnSeePawn`
  (params (Pawn :type "Pawn Object Reference"))
  (set `self.isSeeingPlayer?` true)
  (`self.FollowPlayer`))

(event `FollowPlayer`
  (set `self.canAttack?` true)
  (if (`self.isSeeingPlayer?`)
    (`|AIMoveTo` self (0.0 0.0 0.0) (`GameplayStatics.GetPlayerCharacter` 0) 70.0
      (:`OnSuccess`
        (if (`self.canAttack?`)
          (set `self.canAttack?` false)
          (bind _returnvalue (`self.PlayAnimMontage` "/Game/Game/Animations/ThridPsn_to_MaximoMM_Pistol_Fire_Montage.ThridPsn_to_MaximoMM_Pistol_Fire_Montage"))
          (`KismetSystemLibrary.Delay` _returnvalue)
          (set `self.canAttack?` true))))
    (else
      (set `self.isSeeingPlayer?` false))))

(fn `UserConstructionScript`)